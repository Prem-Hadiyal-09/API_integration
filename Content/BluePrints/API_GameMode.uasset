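; Game mode that fetches articles from a web API and shows them in a scrollable UI list.
; On BeginPlay it shows the cursor, creates the scroll box widget and sends a VaRest GET, whose callback stores the "articles" array and clears a flag.
; A fast looping timer polls that flag, then stops and adds the first five articles as entry widgets with title, description, image URL and link.
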(event `self.ReceiveBeginPlay`
  (set `PlayerController.bShowMouseCursor` true (`GameplayStatics.GetPlayerController` 0))
  (bind _returnvalue (`|CreateWidget` "/Game/UI/ScrollBox_UI.ScrollBox_UI_C"))
  (bind _output_get (set `self.Scroll Box UI Ref` _returnvalue))
  (`UserWidget.AddToViewport` _output_get 0)
  (`self.Get Data From API`)
  (bind _returnvalue_2 (`KismetSystemLibrary.K2_SetTimerDelegate` (delegate `Go`) 0.01 true))
  (set `self.Timer by Event` _returnvalue_2))

(event `Go`
  (if (not (`self.Bool`))
    (`KismetSystemLibrary.K2_ClearAndInvalidateTimerHandle` (`self.Timer by Event`))
    (for _index (range 5)
      (`self.Add_Data` _index))))

(event `Get Data From API`
  (`VaRestSubsystem.CallURL` (subsystem `VaRestSubsystem`) (`self.URL`) "GET" "x_www_form_urlencoded_url" null (delegate `Get Response`)))

(event `Get Response`
  (params (Request :type "VaRestRequestJSON Object Reference"))
  (bind _returnvalue (`VaRestJsonValue.AsObject` (`VaRestRequestJSON.GetResponseValue` Request)))
  (set `self.API_Data` (`VaRestJsonObject.GetArrayField` _returnvalue "articles"))
  (set `self.Bool` false))

(event `Add_Data`
  (params (`API Index` :type Integer))
  (bind _api_data (`self.API_Data`))
  (set `self.Latest_ID` `API Index`)
  (if (< `API Index` (`KismetArrayLibrary.Array_Length` _api_data))
    (bind _returnvalue (`|CreateWidget` "/Game/UI/ListviewDataEntry.ListviewDataEntry_C"))
    (set `self.Listview Data Entry UI Ref` _returnvalue)
    (bind _returnvalue_2 (`VaRestJsonValue.AsObject` (`|GetArrayItem` _api_data `API Index`)))
    (`/Game/UI/ListviewDataEntry.Update UI Data` (`self.Listview Data Entry UI Ref`) (`KismetTextLibrary.Conv_StringToText` (`VaRestJsonObject.GetStringField` _returnvalue_2 "title")) (`KismetTextLibrary.Conv_StringToText` (`VaRestJsonObject.GetStringField` _returnvalue_2 "description")) (`VaRestJsonObject.GetStringField` _returnvalue_2 "urlToImage") (`VaRestJsonObject.GetStringField` _returnvalue_2 "url"))
    (`/Game/UI/ScrollBox_UI.Add Child` (`self.Scroll Box UI Ref`) (`self.Listview Data Entry UI Ref`))))

(fn `UserConstructionScript`)